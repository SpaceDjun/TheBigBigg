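; BP_FlickeringLamp is a greybox lamp actor whose spotlight flickers at random intervals, with occasional effects and sound.
; Tick drives a chain of Delay nodes that toggles SpotLight visibility in a quick double blink after a short random wait.
; A check on Fixed then leads to a longer random delay, an added Niagara component and a flicker cue played at the light's location.
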(event EventBeginPlay)

(event Collision|EventActorBeginOverlap
  (params (OtherActor :type Actor%20Object%20Reference)))

(event EventTick
  (params (DeltaSeconds :type Float%20%28single-precision%29))
  (bind _spotlight (Variables|Default|GetSpotLight))
  (Utilities|FlowControl|Delay (Math|Conversions|ToFloat(Integer) (Math|Random|RandomInteger 2)))
  (Rendering|SetVisibility _spotlight false false)
  (Utilities|FlowControl|Delay 0.2)
  (Rendering|SetVisibility _spotlight true false)
  (Utilities|FlowControl|Delay 0.1)
  (Rendering|SetVisibility _spotlight false false)
  (Utilities|FlowControl|Delay 0.2)
  (Rendering|SetVisibility _spotlight true false)
  (switch Utilities|FlowControl|Switch|SwitchonENiagara_InfiniteLoopDuration "NewEnumerator0"
    (:NewEnumerator0
      (Utilities|FlowControl|Delay (Math|Conversions|ToFloat(Integer) (Math|Random|RandomInteger 10)))
      (AddComponent|AddNiagaraComponent false (Math|Conversions|ToTransform(Vector) "220.000000, 0,490.000000"))
      (Audio|PlaySoundatLocation "/Game/Sound_FX_and_Music/SC_Light_Flicker_Cue.SC_Light_Flicker_Cue" (Transformation|GetWorldLocation _spotlight) "0, 0, 0" 1.0 1.0 0.0 0 0 0 0))))

(fn ConstructionScript)
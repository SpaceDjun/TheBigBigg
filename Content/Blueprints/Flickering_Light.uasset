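; Flickering light actor that blinks its SpotLight off and on in a repeating double flicker.
; Tick drives a chain of Delay nodes that toggle the light's visibility, relying on Delay ignoring re-triggers while pending to pace the pattern.
; A random whole-second Delay ends the chain with nothing after it, so it does not vary the flicker timing.
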(event EventBeginPlay)

(event Collision|EventActorBeginOverlap
  (params (OtherActor :type Actor%20Object%20Reference)))

(event EventTick
  (params (DeltaSeconds :type Float%20%28single-precision%29))
  (bind _spotlight (Variables|Default|GetSpotLight))
  (Utilities|FlowControl|Delay 1.0)
  (Rendering|SetVisibility _spotlight false false)
  (Utilities|FlowControl|Delay 0.2)
  (Rendering|SetVisibility _spotlight true false)
  (Utilities|FlowControl|Delay 0.1)
  (Rendering|SetVisibility _spotlight false false)
  (Utilities|FlowControl|Delay 0.2)
  (Rendering|SetVisibility _spotlight true false)
  (switch Utilities|FlowControl|Switch|SwitchonENiagara_InfiniteLoopDuration "NewEnumerator0"
    (:NewEnumerator0
      (Utilities|FlowControl|Delay (Math|Conversions|ToFloat(Integer) (Math|Random|RandomInteger 10))))))

(fn ConstructionScript)
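; BP_JigSaw is a puzzle prop that opens a jigsaw widget when the player presses Interact nearby.
; Its collision box enables input on overlap and disables it when overlap ends.
; A FlipFlop on Interact alternates between creating the widget with game paused and cursor shown, and removing it to resume play.
; The piece-completion check runs right after opening and triggers nothing.
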(event OnComponentBeginOverlap(CollisionBox)
  (params (OverlappedComponent :type Primitive%20Component%20Object%20Reference) (OtherActor :type Actor%20Object%20Reference) (OtherComp :type Primitive%20Component%20Object%20Reference) (OtherBodyIndex :type Integer) (bFromSweep :type Boolean) (SweepResult :type Hit%20Result%20Structure%20%28by%20ref%29))
  (Utilities|Casting|CastTo OtherActor)
  (Input|EnableInput (Game|GetPlayerController 0)))

(event OnComponentEndOverlap(CollisionBox)
  (params (OverlappedComponent :type Primitive%20Component%20Object%20Reference) (OtherActor :type Actor%20Object%20Reference) (OtherComp :type Primitive%20Component%20Object%20Reference) (OtherBodyIndex :type Integer))
  (Utilities|Casting|CastTo OtherActor)
  (Input|DisableInput (Game|GetPlayerController 0)))

(event Input|ActionEvents|InputActionInteract
  (params (Key :type Key%20Structure))
  (bind _returnvalue (Game|GetPlayerController 0))
  (:Pressed
    (Utilities|FlowControl|FlipFlop
      (:A
        (bind _returnvalue_2 (UserInterface|CreateWidget "/Game/TestLevelPortal/Puzzle/BluePrint/Props/Jigsaw/JigsawWidget.JigsawWidget_C" (Game|GetPlayerController 0)))
        (UserInterface|Viewport|AddtoViewport _returnvalue_2 0)
        (Game|SetGamePaused true)
        (Variables|/Script/Engine.PlayerController|SetbShowMouseCursor _returnvalue true)
        (if (== (Variables|/Game/TestLevelPortal/Puzzle/BluePrint/Props/Jigsaw/JigsawWidget.JigsawWidget_C|GetCorrectlyPlacedPieces _returnvalue_2) (Variables|/Game/TestLevelPortal/Puzzle/BluePrint/Props/Jigsaw/JigsawWidget.JigsawWidget_C|GetNumber%20of%20Pieces _returnvalue_2))
          _))
      (:B
        (Widget|RemovefromParent _returnvalue_2)
        (Game|SetGamePaused false)
        (Variables|/Script/Engine.PlayerController|SetbShowMouseCursor _returnvalue false)))))

(fn ConstructionScript)